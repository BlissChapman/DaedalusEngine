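; Maze cell actor that builds its own walls, optional floor and optional ceiling for one grid square of a maze.
; ConfigCell copies grid position, dimensions, thicknesses and floor/ceiling flags from the owning maze and clears the wall flags.
; GetAdjacentCells fetches the four neighbours from the maze, substituting its placeholder cell beyond the grid edges.
; MakeWalls adds scaled static mesh components, skipping any wall the neighbour already built to avoid duplicates.
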(event EventActorBeginOverlap
  (params (OtherActor :type Actor%20Object%20Reference)))

(event EventTick
  (params (DeltaSeconds :type Float%20%28single-precision%29)))

(fn ConstructionScript)

(fn GetAdjacentCells
  (bind _cellpos (Variables|CellProperties|GetCellPos))
  (bind _cellpos_2 (Variables|CellProperties|GetCellPos))
  (bind _cellpos_3 (Variables|CellProperties|GetCellPos))
  (bind _cellpos_4 (Variables|CellProperties|GetCellPos))
  (bind (_x _y) (Math|Vector2D|BreakVector2D _cellpos_3))
  (bind (_x_2 _y_2) (Math|Vector2D|BreakVector2D _cellpos_4))
  (bind (_x_3 _y_3) (Math|Vector2D|BreakVector2D _cellpos_2))
  (bind (_x_4 _y_4) (Math|Vector2D|BreakVector2D _cellpos))
  (bind _returnvalue (+ _y -1.0))
  (bind _returnvalue_2 (+ _x_2 1.0))
  (bind _returnvalue_3 (+ _x_3 -1.0))
  (bind _returnvalue_4 (+ _y_4 1.0))
  (Variables|Default|SetadjacentCells (Utilities|Array|MakeArray 0 0 0 0))
  (Utilities|FlowControl|Sequence
    (:then_0
      ;[1 1 1] North
      (if (>= _returnvalue_4 (Math|Conversions|ToFloat(Integer) (Variables|/Game/Maze/Blueprints/Daedalus.Daedalus_C|GetgridHeight (Variables|Default|GetMAZE))))
        (Utilities|Array|SetArrayElem (Variables|Default|GetadjacentCells) 0 (Variables|/Game/Maze/Blueprints/Daedalus.Daedalus_C|GetplaceholderCell (Variables|Default|GetMAZE)))
        (else
          (bind _cell (Default|GetCellatCoordinate (Variables|Default|GetMAZE) (Math|Vector2D|MakeVector2D _x_4 _returnvalue_4)))
          (Utilities|Array|SetArrayElem (Variables|Default|GetadjacentCells) 0 _cell))))
    (:then_1
      ;[1 1 1] East
      (if (< _returnvalue_3 0.0)
        (Utilities|Array|SetArrayElem (Variables|Default|GetadjacentCells) 1 (Variables|/Game/Maze/Blueprints/Daedalus.Daedalus_C|GetplaceholderCell (Variables|Default|GetMAZE)))
        (else
          (bind _cell_2 (Default|GetCellatCoordinate (Variables|Default|GetMAZE) (Math|Vector2D|MakeVector2D _returnvalue_3 _y_3)))
          (Utilities|Array|SetArrayElem (Variables|Default|GetadjacentCells) 1 _cell_2))))
    (:then_2
      ;[1 1 1] South
      (if (< _returnvalue 0.0)
        (Utilities|Array|SetArrayElem (Variables|Default|GetadjacentCells) 2 (Variables|/Game/Maze/Blueprints/Daedalus.Daedalus_C|GetplaceholderCell (Variables|Default|GetMAZE)))
        (else
          (bind _cell_3 (Default|GetCellatCoordinate (Variables|Default|GetMAZE) (Math|Vector2D|MakeVector2D _x _returnvalue)))
          (Utilities|Array|SetArrayElem (Variables|Default|GetadjacentCells) 2 _cell_3))))
    (:then_3
      ;[1 1 1] West
      (if (> _returnvalue_2 (Math|Conversions|ToFloat(Integer) (- (Variables|/Game/Maze/Blueprints/Daedalus.Daedalus_C|GetgridWidth (Variables|Default|GetMAZE)) 1)))
        (Utilities|Array|SetArrayElem (Variables|Default|GetadjacentCells) 3 (Variables|/Game/Maze/Blueprints/Daedalus.Daedalus_C|GetplaceholderCell (Variables|Default|GetMAZE)))
        (else
          (bind _cell_4 (Default|GetCellatCoordinate (Variables|Default|GetMAZE) (Math|Vector2D|MakeVector2D _returnvalue_2 _y_2)))
          (Utilities|Array|SetArrayElem (Variables|Default|GetadjacentCells) 3 _cell_4))))))

(fn MakeWalls
  (CallFunction|GetAdjacentCells)
  (Utilities|FlowControl|Sequence
    (:then_0
      ;[1 1 1] Add North Wall if appropriate
      (if (not (Variables|Cell_C|GetsouthWallExists (Utilities|Array|Get(acopy) (Variables|Default|GetadjacentCells))))
        (bind _returnvalue (AddComponent|AddStaticMeshComponent true (Math|Transform|MakeTransform (+ (Transformation|GetWorldLocation (Variables|Default|GetDefaultSceneRoot)) (Math|Vector|MakeVector 0.0 (Variables|CellProperties|Getcell%20Y) (Variables|CellProperties|Getcell%20Z))) "0,90.000000,0.000000" (Variables|CellProperties|GetWallScale))))
        (Variables|Default|SetNorthWall _returnvalue)
        (Variables|CellStates|SetnorthWallExists true)
        (Transformation|SetWorldScale3D _returnvalue (Math|Vector|MakeVector (/ (Variables|CellProperties|GetWallThickness) 1e+01) (/ (Variables|CellProperties|Getcell%20X) 2e+02) (/ (Variables|CellProperties|Getcell%20Z) 1.5e+02)))))
    (:then_1
      ;[1 1 1] Add East Wall if appropriate
      (if (not (Variables|Cell_C|GetwestWallExists (Utilities|Array|Get(acopy) (Variables|Default|GetadjacentCells) 1)))
        (bind _returnvalue_2 (AddComponent|AddStaticMeshComponent true (Math|Transform|MakeTransform (+ (Transformation|GetWorldLocation (Variables|Default|GetDefaultSceneRoot)) (Math|Vector|MakeVector (* (Variables|CellProperties|Getcell%20X) -1.0) 0.0 (Variables|CellProperties|Getcell%20Z))) "0,0.000000, 0" (Variables|CellProperties|GetWallScale))))
        (Variables|Default|SetEastWall _returnvalue_2)
        (Variables|CellStates|SeteastWallExists true)
        (Transformation|SetWorldScale3D _returnvalue_2 (Math|Vector|MakeVector (/ (Variables|CellProperties|GetWallThickness) 1e+01) (/ (Variables|CellProperties|Getcell%20Y) 2e+02) (/ (Variables|CellProperties|Getcell%20Z) 1.5e+02)))))
    (:then_2
      ;[1 1 1] Add South Wall if appropriate
      (if (not (Variables|Cell_C|GetnorthWallExists (Utilities|Array|Get(acopy) (Variables|Default|GetadjacentCells) 2)))
        (bind _returnvalue_3 (AddComponent|AddStaticMeshComponent true (Math|Transform|MakeTransform (+ (Transformation|GetWorldLocation (Variables|Default|GetDefaultSceneRoot)) (Math|Vector|MakeVector 0.0 (* (Variables|CellProperties|Getcell%20Y) -1.0) (Variables|CellProperties|Getcell%20Z))) "0,90.000000, 0" (Variables|CellProperties|GetWallScale))))
        (Variables|Default|SetSouthwall _returnvalue_3)
        (Variables|CellStates|SetsouthWallExists true)
        (Transformation|SetWorldScale3D _returnvalue_3 (Math|Vector|MakeVector (/ (Variables|CellProperties|GetWallThickness) 1e+01) (/ (Variables|CellProperties|Getcell%20X) 2e+02) (/ (Variables|CellProperties|Getcell%20Z) 1.5e+02)))))
    (:then_3
      ;[1 1 1] Add West Wall if appropriate
      (if (not (Variables|Cell_C|GeteastWallExists (Utilities|Array|Get(acopy) (Variables|Default|GetadjacentCells) 3)))
        (bind _returnvalue_4 (AddComponent|AddStaticMeshComponent true (Math|Transform|MakeTransform (+ (Transformation|GetWorldLocation (Variables|Default|GetDefaultSceneRoot)) (Math|Vector|MakeVector (Variables|CellProperties|Getcell%20X) 0.0 (Variables|CellProperties|Getcell%20Z))) "0,0.000000, 0" (Variables|CellProperties|GetWallScale))))
        (Variables|Default|SetWestwall _returnvalue_4)
        (Variables|CellStates|SetwestWallExists true)
        (Transformation|SetWorldScale3D _returnvalue_4 (Math|Vector|MakeVector (/ (Variables|CellProperties|GetWallThickness) 1e+01) (/ (Variables|CellProperties|Getcell%20Y) 2e+02) (/ (Variables|CellProperties|Getcell%20Z) 1.5e+02)))))
    (:then_4
      ;[1 1 1] Create floors
      (if (Variables|CellProperties|GetHasFloor)
        (bind _returnvalue_5 (AddComponent|AddStaticMeshComponent true (Math|Transform|MakeTransform (+ (Math|Vector|MakeVector 0.0 0.0 (- 0.0 (/ (Variables|CellProperties|GetFloorThickness) 2.0))) (Transformation|GetWorldLocation (Variables|Default|GetDefaultSceneRoot))) "90.000000, 0,0.000000" (Variables|CellStates|GetFLOOR_SCALE))))
        (Variables|Default|SetCellFloor _returnvalue_5)
        (Variables|CellStates|Setfloorexists true)
        (Transformation|SetWorldScale3D _returnvalue_5 (Math|Vector|MakeVector (/ (Variables|CellProperties|GetFloorThickness) 1e+01) (/ (Variables|CellProperties|Getcell%20Y) 2e+02) (/ (Variables|CellProperties|Getcell%20X) 2e+02)))))
    (:then_5
      ;[1 1 1] Create Ceilings
      (if (Variables|CellProperties|GetHasCeiling)
        (bind _returnvalue_6 (AddComponent|AddStaticMeshComponent true (Math|Transform|MakeTransform (+ (Math|Vector|MakeVector 0.0 0.0 (+ (* (Variables|CellProperties|Getcell%20Z) 2.0) (/ (Variables|CellProperties|GetCeilingThickness) 2.0))) (Transformation|GetWorldLocation (Variables|Default|GetDefaultSceneRoot))) "90.000000, 0,0.000000" (Variables|CellStates|GetFLOOR_SCALE))))
        (Variables|Default|SetCellFloor _returnvalue_6)
        (Variables|CellStates|Setfloorexists true)
        (Transformation|SetWorldScale3D _returnvalue_6 (Math|Vector|MakeVector (/ (Variables|CellProperties|GetCeilingThickness) 1e+01) (/ (Variables|CellProperties|Getcell%20Y) 2e+02) (/ (Variables|CellProperties|Getcell%20X) 2e+02)))))))

(fn ConfigCell
  (params (Maze :type Daedalus%20Object%20Reference))
  (Variables|Default|SetMAZE Maze)
  (Variables|CellProperties|SetCellPos (Variables|/Game/Maze/Blueprints/Daedalus.Daedalus_C|GetcellPosition (Variables|Default|GetMAZE)))
  (Variables|CellProperties|Setcell%20Y (Variables|/Game/Maze/Blueprints/Daedalus.Daedalus_C|GetCELL_Y (Variables|Default|GetMAZE)))
  (Variables|CellProperties|Setcell%20X (Variables|/Game/Maze/Blueprints/Daedalus.Daedalus_C|GetCELL_X (Variables|Default|GetMAZE)))
  (Variables|CellProperties|Setcell%20Z (Variables|/Game/Maze/Blueprints/Daedalus.Daedalus_C|GetCELL_Z (Variables|Default|GetMAZE)))
  (Variables|CellProperties|SetWallThickness (Variables|/Game/Maze/Blueprints/Daedalus.Daedalus_C|GetWallThickness (Variables|Default|GetMAZE)))
  (Variables|CellProperties|SetFloorThickness (Variables|/Game/Maze/Blueprints/Daedalus.Daedalus_C|GetFloorThickness (Variables|Default|GetMAZE)))
  (Variables|CellProperties|SetCeilingThickness (Variables|/Game/Maze/Blueprints/Daedalus.Daedalus_C|GetCeilingThickness (Variables|Default|GetMAZE)))
  (Variables|CellProperties|SetHasFloor (Variables|/Game/Maze/Blueprints/Daedalus.Daedalus_C|GetHasFloor (Variables|Default|GetMAZE)))
  (Variables|CellProperties|SetHasCeiling (Variables|/Game/Maze/Blueprints/Daedalus.Daedalus_C|GetHasCeiling (Variables|Default|GetMAZE)))
  (Variables|CellStates|SetnorthWallExists false)
  (Variables|CellStates|SetsouthWallExists false)
  (Variables|CellStates|SeteastWallExists false)
  (Variables|CellStates|SetwestWallExists false))